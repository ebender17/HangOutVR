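; Campfire game mode that tracks connected players and spawns a VR or first-person actor for each login.
; BeginPlay caches the level's PlayerStarts, and login and logout add or remove MyPlayerControllers from ConnectedPlayers.
; After a short post-login delay and a DefaultPawnClass check, it spawns BP_MotionController if a headset is enabled, otherwise FirstPersonCharacter.
; Spawns always use the first PlayerStart, and the graph does not possess the spawned actor.
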(event `self.ReceiveBeginPlay`
  (bind _outactors (`GameplayStatics.GetAllActorsOfClass` "/Script/Engine.PlayerStart"))
  (set `self.Player Start` _outactors))

(event `self.K2_PostLogin`
  (params (NewPlayer :type "PlayerController Object Reference"))
  (bind _returnvalue (`self.GetTransform` (`|GetArrayItem` (`self.Player Start`))))
  (bind _asmy_player_controller (cast `/Game/FirstPersonBP/Blueprints/Chat/MyPlayerController` NewPlayer))
  (`KismetArrayLibrary.Array_Add` (`self.Connected Players`) _asmy_player_controller)
  (`KismetSystemLibrary.Delay` 0.2)
  (if (== (`self.DefaultPawnClass`) null)
    (if (`HeadMountedDisplayFunctionLibrary.IsHeadMountedDisplayEnabled`)
      (`|SpawnActorFromClass` "/Game/VirtualRealityBP/Blueprints/BP_MotionController.BP_MotionController_C" _returnvalue "AdjustIfPossibleButAlwaysSpawn" "OverrideRootScale" null "Left" null)
      (else
        (`|SpawnActorFromClass` "/Game/FirstPersonBP/Blueprints/FirstPersonCharacter.FirstPersonCharacter_C" _returnvalue "AdjustIfPossibleButAlwaysSpawn" "OverrideRootScale" null null)))))

(event `self.K2_OnLogout`
  (params (ExitingController :type "Controller Object Reference"))
  (bind _asmy_player_controller (cast `/Game/FirstPersonBP/Blueprints/Chat/MyPlayerController` ExitingController))
  (`KismetArrayLibrary.Array_RemoveItem` (`self.Connected Players`) _asmy_player_controller))

(fn `UserConstructionScript`)